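; Demo actor for a compute shader with variable-length output, visualized as debug arrows.
; Each Tick, while no dispatch is pending, it line-traces toward Target and passes its location and the hit normal to ExecuteVariableOutputComputeShader, requesting a fixed output count.
; The asynchronous completion draws an arrow from the actor to each returned point.
; The Completed flag gates Tick, preventing overlapping dispatches.
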(event `self.ReceiveTick`
  (params (DeltaSeconds :type "Float (single-precision)"))
  (bind _returnvalue (`KismetMathLibrary.Conv_ColorToLinearColor` (`self.Color`)))
  (if (`self.Completed`)
    (bind (_outhit _returnvalue_2) (`KismetSystemLibrary.LineTraceSingle` :`Start` (`self.K2_GetActorLocation`) :`End` (`self.K2_GetActorLocation` (`self.Target`)) :`TraceChannel` "TraceTypeQuery1" :`DrawDebugType` "ForOneFrame"))
    (if _returnvalue_2
      (bind _value (`VariableOutput_AsyncExecution.ExecuteVariableOutputComputeShader` (`self.K2_GetActorLocation`) (`.Normal` (`GameplayStatics.BreakHitResult` _outhit)) 15)
        (:`then`
          (set `self.Completed` false))
        (:`Completed`
          (for _array_element _value
            (`KismetMathLibrary.LinearColor_SetRandomHue` _returnvalue)
            (`KismetSystemLibrary.DrawDebugArrow` (`self.K2_GetActorLocation`) _array_element 5.0 _returnvalue 0.1 5.0))
          (set `self.Completed` true))))))

(fn `UserConstructionScript`)