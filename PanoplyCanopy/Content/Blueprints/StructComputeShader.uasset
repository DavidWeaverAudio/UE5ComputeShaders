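; Test actor that runs a variable-input compute shader on an array of random points and visualizes the returned result.
; Tick, when no job is pending, randomizes the points on the Z=0 plane, draws them, then dispatches them with the actor's location.
; The async node returns an index, whose point is highlighted larger in pink.
; A Completed flag gates Tick to one dispatch at a time.
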(event `self.ReceiveBeginPlay`
  (set `self.Completed` true))

(event `self.ReceiveTick`
  (params (DeltaSeconds :type "Float (single-precision)"))
  (bind _vectarr (`self.VectArr`))
  (if (`self.Completed`)
    (for (_array_element _array_index) (`self.VectArr`)
      (`KismetArrayLibrary.Array_Set` (`self.VectArr`) _array_index (`KismetMathLibrary.MakeVector` (`KismetMathLibrary.RandomFloatInRange` 0.0 5000.0) (`KismetMathLibrary.RandomFloatInRange` 0.0 5000.0) (`KismetMathLibrary.RandomFloatInRange` 0.0)))
      (`KismetSystemLibrary.DrawDebugPoint` _array_element 50.0 (struct :`R` 0.42557 :`G` 1.0 :`B` 0.960176 :`A` 1.0) 0.2))
    (bind _value (`VariableInput_AsyncExecution.ExecuteVariableInputComputeShader` _vectarr (`self.K2_GetActorLocation`))
      (:`then`
        (set `self.Completed` false))
      (:`Completed`
        (if (`KismetArrayLibrary.Array_IsValidIndex` _vectarr _value)
          (`KismetSystemLibrary.DrawDebugPoint` (`|GetArrayItem` _vectarr _value) 100.0 (struct :`R` 1.0 :`G` 0.277711 :`B` 0.67776 :`A` 1.0) 1.0))
        (set `self.Completed` true)))))

(fn `UserConstructionScript`)