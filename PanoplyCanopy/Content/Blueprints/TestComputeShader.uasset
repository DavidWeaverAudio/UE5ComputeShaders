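; Test actor that runs a custom compute shader to measure the distance between a vector and a target actor's location.
; Tick dispatches the asynchronous shader call only when the previous one has completed, using a Completed flag as a gate.
; On completion it prints both inputs with the GPU distance next to a CPU-computed distance for comparison, then reopens the gate.
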(event `self.ReceiveBeginPlay`
  (set `self.Completed` true))

(event `self.ReceiveTick`
  (params (DeltaSeconds :type "Float (single-precision)"))
  (bind _arg_1 (`self.Arg 1`))
  (bind _returnvalue (`self.K2_GetActorLocation` (`self.Target`)))
  (if (`self.Completed`)
    (bind _value (`MySimpleComputeShaderLibrary_AsyncExecution.ExecuteBaseComputeShader` _arg_1 _returnvalue)
      (:`then`
        (set `self.Completed` false))
      (:`Completed`
        (`KismetSystemLibrary.PrintString` (`KismetTextLibrary.Conv_TextToString` (`|FormatText` "MyVector: {MyVect} \nOtherVec : {OtherVec} \nDist GPU: {Distance} \nDistCPU : {DistCPU}" (`KismetStringLibrary.Conv_Vector3fToString` _arg_1) (`KismetStringLibrary.Conv_Vector3fToString` _returnvalue) _value (`KismetMathLibrary.Vector_Distance` _arg_1 _returnvalue))) true true (struct :`G` 0.66 :`B` 1.0 :`A` 1.0) 2.0 "Metric")
        (set `self.Completed` true)))))

(fn `UserConstructionScript`)